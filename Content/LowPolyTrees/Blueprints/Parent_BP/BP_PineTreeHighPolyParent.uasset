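; Parent Blueprint for high-poly pine trees in the LowPolyTrees set, configuring the Tree component's size and leaf color.
; The Construction Script optionally overrides world scale with a single Scale value on the axes chosen by ScaleType, keeping the others as they are.
; It then sets material slot 0 to a green, cherry, faded or autumn leaf material based on Type.
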(fn `UserConstructionScript`
  (bind _scale (`self.Scale`))
  (bind _scale_2 (`self.Scale`))
  (bind _scale_3 (`self.Scale`))
  (bind _scale_4 (`self.Scale`))
  (bind _x (.x (`SceneComponent.K2_GetComponentScale` (`self.Tree`))))
  (bind _y (.y (`SceneComponent.K2_GetComponentScale` (`self.Tree`))))
  (bind _z (.z (`SceneComponent.K2_GetComponentScale` (`self.Tree`))))
  (if (`self.Set Scale`)
    (switch `/Game/LowPolyTrees/Blueprints/Parent_BP/E_ScaleType` (`self.Scale Type`)
      (:`NewEnumerator0`
        (`SceneComponent.SetWorldScale3D` (`self.Tree`) (`KismetMathLibrary.MakeVector` (`self.Scale`) _y _z)))
      (:`NewEnumerator1`
        (`SceneComponent.SetWorldScale3D` (`self.Tree`) (`KismetMathLibrary.MakeVector` _x (`self.Scale`) _z)))
      (:`NewEnumerator2`
        (`SceneComponent.SetWorldScale3D` (`self.Tree`) (`KismetMathLibrary.MakeVector` _x _y (`self.Scale`))))
      (:`NewEnumerator3`
        (`SceneComponent.SetWorldScale3D` (`self.Tree`) (`KismetMathLibrary.MakeVector` _scale_2 _scale_2 _z)))
      (:`NewEnumerator4`
        (`SceneComponent.SetWorldScale3D` (`self.Tree`) (`KismetMathLibrary.MakeVector` _scale _y _scale)))
      (:`NewEnumerator5`
        (`SceneComponent.SetWorldScale3D` (`self.Tree`) (`KismetMathLibrary.MakeVector` _x _scale_4 _scale_4)))
      (:`NewEnumerator6`
        (`SceneComponent.SetWorldScale3D` (`self.Tree`) (`KismetMathLibrary.MakeVector` _scale_3 _scale_3 _scale_3)))))
  (switch `/Game/LowPolyTrees/Blueprints/Parent_BP/E_Type` (`self.Type`)
    (:`NewEnumerator0`
      (`PrimitiveComponent.SetMaterial` (`self.Tree`) 0 "/Game/LowPolyTrees/Materials/M_Leaves_Green.M_Leaves_Green"))
    (:`NewEnumerator1`
      (`PrimitiveComponent.SetMaterial` (`self.Tree`) 0 "/Game/LowPolyTrees/Materials/M_Leaves_Cherry.M_Leaves_Cherry"))
    (:`NewEnumerator2`
      (`PrimitiveComponent.SetMaterial` (`self.Tree`) 0 "/Game/LowPolyTrees/Materials/M_Leaves_Faded.M_Leaves_Faded"))
    (:`NewEnumerator3`
      (`PrimitiveComponent.SetMaterial` (`self.Tree`) 0 "/Game/LowPolyTrees/Materials/M_Leaves_Autumn.M_Leaves_Autumn"))))